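; Player Blueprint for a Crossy Road-style chicken game, handling hop movement, death, scoring, HUD creation and game start/restart state.
; WASD presses turn and crouch the chicken, releases play timeline hops, and forward hops score when X exceeds all recorded positions.
; Tick auto-scrolls the camera, faster when the chicken is far ahead, ending the game if it falls behind.
; Tick also carries the chicken on logs and drowns it after a short count on water.
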(event `self.ReceiveBeginPlay`
  (bind _returnvalue (`|CreateWidget` "/Game/Blueprints/HUD.HUD_C"))
  (bind _output_get (set `self.Score_Ref` _returnvalue))
  (`UserWidget.AddToViewport` _output_get 0))

(event `self.ReceiveTick`
  (params (DeltaSeconds :type "Float (single-precision)"))
  (bind (_logspeed_x _logspeed_y) (`KismetMathLibrary.BreakVector` (`self.LogSpeed`)))
  (bind (_logspeed_x_2 _logspeed_y_2) (`KismetMathLibrary.BreakVector` (`self.LogSpeed`)))
  (bind _returnvalue (`KismetMathLibrary.Abs` (- (.x (`SceneComponent.K2_GetComponentLocation` (`self.RotateChicken`))) (.x (`SceneComponent.K2_GetComponentLocation` (`self.Camera`))))))
  (if (not (`self.CannotMove`))
    (`|ExecutionSequence`
      (:`then_0`
        (`/Engine/EditorBlueprintResources/StandardMacros.CompareFloat` _returnvalue 700.0
          (:`>`
            (`SceneComponent.K2_AddLocalOffset` (`self.MoveCameraForward`) (`self.SpeedUp`) false false))
          (:`==`
            (`SceneComponent.K2_AddLocalOffset` (`self.MoveCameraForward`) (`self.NormalSpeed`) false false :!label _label)
            (`/Engine/EditorBlueprintResources/StandardMacros.CompareFloat` _returnvalue 160.0
              (:`==`
                _)
              (:`<`
                _))
            (set `self.CannotMove` true)
            (`self.GameEnded`))
          (:`<`
            (goto _label))))
      (:`then_1`
        (if (`self.ChickenOnLog`)
          (if (`self.MovedUp`)
            (`SceneComponent.K2_AddLocalOffset` (`self.RotateChicken`) (`self.LogSpeed`) false false)
            (elif (`self.MovedBack`)
              (`SceneComponent.K2_AddLocalOffset` (`self.RotateChicken`) (`KismetMathLibrary.NegateVector` (`self.LogSpeed`)) false false)
              (elif (`self.MovedRight`)
                (`SceneComponent.K2_AddLocalOffset` (`self.RotateChicken`) (`KismetMathLibrary.MakeVector` _logspeed_y_2) false false)
                (elif (`self.MovedLeft`)
                  (bind _result (`/Engine/EditorBlueprintResources/StandardMacros.NegateFloat` _logspeed_y)
                    (:`  `
                      (`SceneComponent.K2_AddLocalOffset` (`self.RotateChicken`) (`KismetMathLibrary.MakeVector` _result) false false)))))))
          (elif (`self.IsOnLilyPad`)
            _
            (elif (`self.IsOnWater`)
              (set `self.Death timer` (+ (`self.Death timer`) 1))
              (if (>= (`self.Death timer`) 30)
                (`GameplayStatics.PlaySound2D` "/Game/Sounds/watersplashlow_Cue.watersplashlow_Cue" 1.0 1.0 0.0 null null)
                (set `self.CannotMove` true)
                (`self.GameEnded`)
                (set `self.IsOnWater` false)))))))))

(event `Key|D`
  (params (Key :type "Key Structure"))
  (bind (_returnvalue_x _returnvalue_y) (`KismetMathLibrary.BreakVector` (`SceneComponent.K2_GetComponentLocation` (`self.RotateChicken`))))
  (bind (_returnvalue_x_2 _returnvalue_y_2) (`KismetMathLibrary.BreakVector` (`SceneComponent.K2_GetComponentLocation` (`self.RotateChicken`))))
  (:`Pressed`
    (if (not (`self.CannotMove`))
      (set `self.Released` false)
      (if (`self.MovedRight`)
        (bind (_direction _newtrack_0) (`Timeline|Crouch` :!via `PlayFromStart` :!label _label_2)
          (:`Update`
            (if (`self.Released`)
              (goto _label_2 :!via `Stop`)
              (else
                (`SceneComponent.K2_AddLocalOffset` (`self.RotateChicken`) (+ _newtrack_0 (`self.CrouchChicken`)) false false)))))
        (else
          (if (`self.MovedLeft`)
            (`SceneComponent.K2_AddLocalRotation` (`self.RotateChicken`) (struct :`Yaw` 180.0) false false)
            (elif (`self.MovedUp`)
              (`SceneComponent.K2_AddLocalRotation` (`self.RotateChicken`) (struct :`Yaw` 90.0) false false)
              (elif (`self.MovedBack`)
                (`SceneComponent.K2_AddLocalRotation` (`self.RotateChicken`) (struct :`Yaw` -90.0) false false)
                (else
                  (`SceneComponent.K2_AddLocalRotation` (`self.RotateChicken`) (struct :`Yaw` 90.0) false false)))))
          (set `self.MovedRight` true)
          (set `self.MovedLeft` false)
          (set `self.MovedUp` false)
          (set `self.MovedBack` false)
          (goto _label_2 :!via `PlayFromStart`)))))
  (:`Released`
    (set `self.Released` true)
    (if (not (`self.CannotMove`))
      (`self.Play Cluck`)
      (`SceneComponent.K2_SetWorldLocation` (`self.RotateChicken`) (`KismetMathLibrary.MakeVector` _returnvalue_x_2 _returnvalue_y_2 91.0) false false)
      (bind (_direction_2 _newtrack_0_2) (`Timeline|Move Chicken Up` :!via `PlayFromStart` :!label _label_3)
        (:`Update`
          (`SceneComponent.K2_AddLocalOffset` (`self.RotateChicken`) (+ _newtrack_0_2 (`self.ChickenUp`)) false false))
        (:`Finished`
          (bind (_direction_3 _newtrack_0_3) (`Timeline|Move Chicken Down` :!via `PlayFromStart`)
            (:`Update`
              (`SceneComponent.K2_AddLocalOffset` (`self.RotateChicken`) (+ _newtrack_0_3 (`self.ChickenDown`)) false false))
            (:`Finished`
              (`SceneComponent.K2_SetWorldLocation` (`self.RotateChicken`) (`KismetMathLibrary.MakeVector` _returnvalue_x _returnvalue_y 91.0) false false))))))))

(event `Key|A`
  (params (Key :type "Key Structure"))
  (bind (_returnvalue_x _returnvalue_y) (`KismetMathLibrary.BreakVector` (`SceneComponent.K2_GetComponentLocation` (`self.RotateChicken`))))
  (:`Pressed`
    (if (not (`self.CannotMove`))
      (set `self.Released` false)
      (if (`self.MovedLeft`)
        (goto _label_2 :!via `PlayFromStart`)
        (else
          (if (`self.MovedRight`)
            (`SceneComponent.K2_AddLocalRotation` (`self.RotateChicken`) (struct :`Yaw` -180.0) false false)
            (elif (`self.MovedUp`)
              (`SceneComponent.K2_AddLocalRotation` (`self.RotateChicken`) (struct :`Yaw` -90.0) false false)
              (elif (`self.MovedBack`)
                (`SceneComponent.K2_AddLocalRotation` (`self.RotateChicken`) (struct :`Yaw` 90.0) false false)
                (else
                  (`SceneComponent.K2_AddLocalRotation` (`self.RotateChicken`) (struct :`Yaw` -90.0) false false)))))
          (set `self.MovedRight` false)
          (set `self.MovedLeft` true)
          (set `self.MovedUp` false)
          (set `self.MovedBack` false)
          (goto _label_2 :!via `PlayFromStart`)))))
  (:`Released`
    (set `self.Released` true)
    (if (not (`self.CannotMove`))
      (`self.Play Cluck`)
      (`SceneComponent.K2_SetWorldLocation` (`self.RotateChicken`) (`KismetMathLibrary.MakeVector` _returnvalue_x _returnvalue_y 91.0) false false)
      (goto _label_3 :!via `PlayFromStart`))))

(event `Key|S`
  (params (Key :type "Key Structure"))
  (bind (_returnvalue_x _returnvalue_y) (`KismetMathLibrary.BreakVector` (`SceneComponent.K2_GetComponentLocation` (`self.RotateChicken`))))
  (:`Pressed`
    (if (not (`self.CannotMove`))
      (set `self.Released` false)
      (if (`self.MovedBack`)
        (goto _label_2 :!via `PlayFromStart`)
        (else
          (if (`self.MovedRight`)
            (`SceneComponent.K2_AddLocalRotation` (`self.RotateChicken`) (struct :`Yaw` 90.0) false false)
            (elif (`self.MovedUp`)
              (`SceneComponent.K2_AddLocalRotation` (`self.RotateChicken`) (struct :`Yaw` 180.0) false false)
              (elif (`self.MovedLeft`)
                (`SceneComponent.K2_AddLocalRotation` (`self.RotateChicken`) (struct :`Yaw` -90.0) false false)
                (else
                  (`SceneComponent.K2_AddLocalRotation` (`self.RotateChicken`) (struct :`Yaw` 180.0) false false)))))
          (set `self.MovedRight` false)
          (set `self.MovedLeft` false)
          (set `self.MovedUp` false)
          (set `self.MovedBack` true)
          (goto _label_2 :!via `PlayFromStart`)))))
  (:`Released`
    (set `self.Released` true)
    (if (not (`self.CannotMove`))
      (`self.Play Cluck`)
      (`SceneComponent.K2_SetWorldLocation` (`self.RotateChicken`) (`KismetMathLibrary.MakeVector` _returnvalue_x _returnvalue_y 91.0) false false)
      (goto _label_3 :!via `PlayFromStart`))))

(event `Key|W`
  (params (Key :type "Key Structure"))
  (bind _returnvalue_x (`KismetMathLibrary.BreakVector` (`SceneComponent.K2_GetComponentLocation` (`self.RotateChicken`))))
  (bind (_returnvalue_x_2 _returnvalue_y) (`KismetMathLibrary.BreakVector` (`SceneComponent.K2_GetComponentLocation` (`self.RotateChicken`))))
  (bind (_returnvalue_x_3 _returnvalue_y_2) (`KismetMathLibrary.BreakVector` (`SceneComponent.K2_GetComponentLocation` (`self.RotateChicken`))))
  (:`Pressed`
    (if (not (`self.CannotMove`))
      (set `self.Released` false)
      (if (`self.MovedUp`)
        (goto _label_2 :!via `PlayFromStart`)
        (else
          (if (`self.MovedRight`)
            (`SceneComponent.K2_AddLocalRotation` (`self.RotateChicken`) (struct :`Yaw` -90.0) false false)
            (elif (`self.MovedBack`)
              (`SceneComponent.K2_AddLocalRotation` (`self.RotateChicken`) (struct :`Yaw` -180.0) false false)
              (elif (`self.MovedLeft`)
                (`SceneComponent.K2_AddLocalRotation` (`self.RotateChicken`) (struct :`Yaw` 90.0) false false)
                (else
                  (`SceneComponent.K2_AddLocalRotation` :`self` (`self.RotateChicken`))))))
          (set `self.MovedRight` false)
          (set `self.MovedLeft` false)
          (set `self.MovedUp` true)
          (set `self.MovedBack` false)
          (goto _label_2 :!via `PlayFromStart`)))))
  (:`Released`
    (set `self.Released` true)
    (if (not (`self.CannotMove`))
      (`self.Play Cluck`)
      (`SceneComponent.K2_SetWorldLocation` (`self.RotateChicken`) (`KismetMathLibrary.MakeVector` _returnvalue_x_3 _returnvalue_y_2 91.0) false false)
      (bind (_direction _newtrack_0) (`Timeline|Timeline_0` :!via `PlayFromStart`)
        (:`Update`
          (`SceneComponent.K2_AddLocalOffset` (`self.RotateChicken`) (+ _newtrack_0 (`self.ChickenUp`)) false false))
        (:`Finished`
          (bind (_direction_2 _newtrack_0_2) (`Timeline|Timeline_1` :!via `PlayFromStart`)
            (:`Update`
              (`SceneComponent.K2_AddLocalOffset` (`self.RotateChicken`) (+ _newtrack_0_2 (`self.ChickenDown`)) false false))
            (:`Finished`
              (`SceneComponent.K2_SetWorldLocation` (`self.RotateChicken`) (`KismetMathLibrary.MakeVector` _returnvalue_x_2 _returnvalue_y 91.0) false false)
              (set `self.X_Val` (`KismetMathLibrary.FTrunc` _returnvalue_x))
              (for _array_element (`self.X_Locations`)
                (if (<= (`self.X_Val`) _array_element)
                  (set `self.LoopBroken` true)
                  (break)))
              (if (`self.LoopBroken`)
                (set `self.LoopBroken` false)
                (else
                  (set `self.Score` (+ (`self.Score`) 1))
                  (if (> (`self.Score`) (`self.HighScore`))
                    (set `self.NewHighScore` true)
                    (set `self.HighScore` (`self.Score`))
                    (`KismetArrayLibrary.Array_Add` (`self.X_Locations`) (`self.X_Val`))))))))))))

(fn `GameEnded`
  (`GameplayStatics.PlaySound2D` "/Game/Sounds/chickendeath_Cue.chickendeath_Cue" 1.0 1.0 0.0 null null)
  (set `self.ShowRestartButton` true)
  (set `self.ChickenDead` true)
  (`GameplayStatics.PlaySound2D` "/Game/Sounds/playerdie_Cue.playerdie_Cue" 1.0 1.0 0.0 null null))

(fn `Play Cluck`
  (`|MultiGate` true
    (:`Out 0`
      (`GameplayStatics.PlaySound2D` "/Game/Sounds/chickencluck.chickencluck" 1.0 1.0 0.0 null null))))

(fn `RestartGame`
  (set `self.ShowRestartButton` false)
  (set `self.NewHighScore` false)
  (`SceneComponent.SetVisibility` (`self.Chicken`) true false)
  (`SceneComponent.K2_AddLocalTransform` (`self.RotateChicken`) (`KismetMathLibrary.MakeTransform` (0.0 0.0 0.0) (struct) (2.25 2.25 2.25)) false false)
  (set `self.ChickenDead` false)
  (set `self.Score` 0)
  (set `self.Coins` 0)
  (`KismetArrayLibrary.Array_Clear` (`self.X_Locations`)))

(fn `StartGame`
  (set `self.ShowStartButton` false)
  (set `self.CannotMove` false)
  (set `self.ShowScore` true))

(fn `UserConstructionScript`)