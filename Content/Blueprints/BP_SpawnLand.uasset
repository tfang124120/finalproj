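; Endless lane generator for a Crossy Road-style chicken game, spawning railroad, road, grass and water strips.
; Each strip chains off the previous SpawnPoint, using random MultiGates and last-type flags to add road lines or water runs and avoid repeated grass.
; Grass drops out from score 50, and old pieces are destroyed once the land count reaches 20.
; Tick watches the player's Restarting flag to rebuild the land and reset the player.
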(event `self.ReceiveBeginPlay`
  (`self.SpawnInitialLand`))

(event `self.ReceiveTick`
  (params (DeltaSeconds :type "Float (single-precision)"))
  (if (not (`self.HasResetted`))
    (bind _asbp_player (cast `/Game/Blueprints/BP_Player` (`GameplayStatics.GetPlayerCharacter` 0)))
    (if (`/Game/Blueprints/BP_Player.Restarting` _asbp_player)
      (`self.DeleteLand`)
      (set `self.LandCount` 0)
      (set `self.Railroadgen` false)
      (set `self.RoadGen` false)
      (set `self.GrassGen` false)
      (set `self.WaterGen` false)
      (set `self.SpawnPlatformSpawned` false)
      (set `self.FirstLandSpawned` false)
      (`self.SpawnInitialLand`)
      (`SceneComponent.SetVisibility` (`/Game/Blueprints/BP_Player.Chicken` _asbp_player) true false)
      (`SceneComponent.K2_SetWorldLocation` (`/Game/Blueprints/BP_Player.MoveCameraForward` _asbp_player) (-500.0 1450.0 900.0) false false)
      (`SceneComponent.K2_SetWorldLocation` (`/Game/Blueprints/BP_Player.RotateChicken` _asbp_player) (122.0 1450.0 100.0) false false)
      (`KismetSystemLibrary.Delay` 2.0)
      (set `/Game/Blueprints/BP_Player.Restarting` false _asbp_player)
      (set `/Game/Blueprints/BP_Player.CannotMove` false _asbp_player)
      (set `self.HasResetted` false))))

(fn `DeleteLand`
  (for _array_element (`self.LandArray`)
    (`/Engine/EditorBlueprintResources/StandardMacros.IsValid` _array_element
      (:`Is Valid`
        (`self.K2_DestroyActor` _array_element))))
  (`self.K2_DestroyActor` (`self.SpawnPlatform`))
  (set `self.HasResetted` true))

(fn `Spawn_Land`
  (params (`Spawn Location` :type "Vector Structure"))
  (bind _asbp_player (cast `/Game/Blueprints/BP_Player` (`GameplayStatics.GetPlayerCharacter` 0)))
  (if (< (`/Game/Blueprints/BP_Player.Score` _asbp_player) 50)
    (`|MultiGate` true
      (:`Out 0`
        (bind _returnvalue (`|SpawnActorFromClass` "/Game/Blueprints/BP_RailRoad.BP_RailRoad_C" (`KismetMathLibrary.MakeTransform` `Spawn Location`) "Undefined" "OverrideRootScale" null null :!label _label))
        (bind _output_get (set `self.New Railroad` _returnvalue))
        (set `/Game/Blueprints/BP_RailRoad.RailroadSpawner` self _output_get)
        (`KismetArrayLibrary.Array_Add` (`self.LandArray`) (`self.New Railroad`))
        (set `self.Railroadgen` true)
        (set `self.RoadGen` false)
        (set `self.GrassGen` false))
      (:`Out 1`
        (if (or (`self.Railroadgen`) (`self.GrassGen`) (`self.WaterGen`)) :!label _label_2
          (bind _returnvalue_2 (`|SpawnActorFromClass` "/Game/Blueprints/BP_SingleRoad.BP_SingleRoad_C" (`KismetMathLibrary.MakeTransform` `Spawn Location`) "Undefined" "OverrideRootScale" null null :!label _label_3))
          (bind _output_get_2 (set `self.New Road` _returnvalue_2))
          (set `/Game/Blueprints/BP_SingleRoad.RoadSpawner` self _output_get_2)
          (`KismetArrayLibrary.Array_Add` (`self.LandArray`) (`self.New Road`))
          (set `self.RoadGen` true)
          (set `self.Railroadgen` false)
          (set `self.GrassGen` false)
          (set `self.WaterGen` false)
          (elif (`self.FirstLandSpawned`)
            (bind _returnvalue_3 (`|SpawnActorFromClass` "/Game/Blueprints/BP_RoadLine.BP_RoadLine_C" (`KismetMathLibrary.MakeTransform` `Spawn Location`) "Undefined" "OverrideRootScale" null null))
            (set `self.New RoadLine` _returnvalue_3)
            (`KismetArrayLibrary.Array_Add` (`self.LandArray`) (`self.New RoadLine`))
            (bind _returnvalue_4 (`|SpawnActorFromClass` "/Game/Blueprints/BP_SingleRoad.BP_SingleRoad_C" (`KismetMathLibrary.MakeTransform` (`SceneComponent.K2_GetComponentLocation` (`/Game/Blueprints/BP_RoadLine.SpawnPoint` (`self.New RoadLine`)))) "Undefined" "OverrideRootScale" null null))
            (bind _output_get_3 (set `self.New Road` _returnvalue_4))
            (set `/Game/Blueprints/BP_SingleRoad.RoadSpawner` self _output_get_3)
            (`KismetArrayLibrary.Array_Add` (`self.LandArray`) (`self.New Road`))
            (set `self.RoadGen` true)
            (set `self.Railroadgen` false)
            (set `self.GrassGen` false)
            (set `self.WaterGen` false)
            (else
              (goto _label_3)))))
      (:`Out 2`
        (goto _label_2))
      (:`Out 3`
        (if (`self.GrassGen`)
          (`|MultiGate` true
            (:`Out 0`
              (goto _label))
            (:`Out 1`
              (goto _label_2))
            (:`Out 2`
              (bind _returnvalue_5 (`|SpawnActorFromClass` "/Game/Blueprints/BP_Water.BP_Water_C" (`KismetMathLibrary.MakeTransform` `Spawn Location`) "Undefined" "OverrideRootScale" null null :!label _label_4))
              (bind _output_get_4 (set `self.New Water` _returnvalue_5))
              (set `/Game/Blueprints/BP_Water.Water Spawner` self _output_get_4)
              (`KismetArrayLibrary.Array_Add` (`self.LandArray`) (`self.New Water`))
              (for _ (range (+ (`KismetMathLibrary.RandomIntegerInRange` 1 3) 1))
                (bind _returnvalue_6 (`|SpawnActorFromClass` "/Game/Blueprints/BP_Water.BP_Water_C" (`KismetMathLibrary.MakeTransform` (`SceneComponent.K2_GetComponentLocation` (`/Game/Blueprints/BP_Water.SpawnPoint` (`self.New Water`)))) "Undefined" "OverrideRootScale" null null))
                (bind _output_get_5 (set `self.New Water` _returnvalue_6))
                (set `/Game/Blueprints/BP_Water.Water Spawner` self _output_get_5)
                (`KismetArrayLibrary.Array_Add` (`self.LandArray`) (`self.New Water`)))
              (set `self.Railroadgen` false)
              (set `self.RoadGen` false)
              (set `self.GrassGen` false)
              (set `self.WaterGen` true)))
          (else
            (bind _returnvalue_7 (`|SpawnActorFromClass` "/Game/Blueprints/BP_Grass.BP_Grass_C" (`KismetMathLibrary.MakeTransform` `Spawn Location`) "Undefined" "OverrideRootScale" null null))
            (bind _output_get_6 (set `self.New Grass` _returnvalue_7))
            (set `/Game/Blueprints/BP_Grass.GrassSpawner` self _output_get_6)
            (`KismetArrayLibrary.Array_Add` (`self.LandArray`) (`self.New Grass`))
            (set `self.Railroadgen` false)
            (set `self.RoadGen` false)
            (set `self.GrassGen` true)
            (set `self.WaterGen` false))))
      (:`Out 4`
        (if (`self.WaterGen`)
          (goto _label_3)
          (else
            (goto _label_4)))))
    (else
      (`|MultiGate` true
        (:`Out 0`
          (goto _label))
        (:`Out 1`
          (goto _label_2))
        (:`Out 2`
          (goto _label_4))))))

(fn `Spawn_Land at Spawn Point`
  (if (`self.RoadGen`)
    (`self.Spawn_Land` (`SceneComponent.K2_GetComponentLocation` (`/Game/Blueprints/BP_SingleRoad.SpawnPoint` (`self.New Road`))))
    (if (== (`self.LandCount`) 20) :!label _label
      (`self.K2_DestroyActor` (`|GetArrayItem` (`self.LandArray`) (`self.ArrayCount`)))
      (set `self.ArrayCount` (+ (`self.ArrayCount`) 1))
      (else
        (set `self.LandCount` (+ (`self.LandCount`) 1))))
    (elif (`self.Railroadgen`)
      (`self.Spawn_Land` (`SceneComponent.K2_GetComponentLocation` (`/Game/Blueprints/BP_RailRoad.SpawnPoint` (`self.New Railroad`))))
      (goto _label)
      (elif (`self.GrassGen`)
        (`self.Spawn_Land` (`SceneComponent.K2_GetComponentLocation` (`/Game/Blueprints/BP_Grass.SpawnPoint` (`self.New Grass`))))
        (goto _label)
        (elif (`self.WaterGen`)
          (`self.Spawn_Land` (`SceneComponent.K2_GetComponentLocation` (`/Game/Blueprints/BP_Water.SpawnPoint` (`self.New Water`))))
          (goto _label)
          (elif (`self.SpawnPlatformSpawned`)
            (`self.Spawn_Land` (`SceneComponent.K2_GetComponentLocation` (`/Game/Blueprints/BP_SpawnPlatform.SpawnPoint` (`self.SpawnPlatform`))))
            (goto _label)))))))

(fn `SpawnInitialLand`
  (for _ (range 14)
    (if (`self.SpawnPlatformSpawned`)
      (`self.Spawn_Land at Spawn Point`)
      (set `self.FirstLandSpawned` true)
      (else
        (bind _returnvalue (`|SpawnActorFromClass` "/Game/Blueprints/BP_SpawnPlatform.BP_SpawnPlatform_C" (`KismetMathLibrary.MakeTransform` (0.0 0.0 0.0)) "Undefined" "OverrideRootScale" null null))
        (set `self.SpawnPlatform` _returnvalue)
        (set `self.SpawnPlatformSpawned` true)))))

(fn `UserConstructionScript`)