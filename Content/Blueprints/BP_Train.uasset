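; BP_Train is a moving train hazard that ends the game when it hits a living player chicken.
; Tick shifts the Train component by a fixed local Z offset each frame, not scaled by delta time, while RailroadRef is valid.
; It destroys that component past a world Y limit or when the player is restarting.
; A CollisionBox overlap with a live BP_Player blocks its movement and calls GameEnded.
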(event `self.ReceiveBeginPlay`)

(event `self.ReceiveTick`
  (params (DeltaSeconds :type "Float (single-precision)"))
  (bind (_returnvalue_x _returnvalue_y) (`KismetMathLibrary.BreakVector` (`SceneComponent.K2_GetComponentLocation` (`self.Train`))))
  (if (not (`self.TrainDestroyed`))
    (bind _asbp_player (cast `/Game/Blueprints/BP_Player` (`GameplayStatics.GetPlayerCharacter` 0)))
    (if (`/Game/Blueprints/BP_Player.Restarting` _asbp_player)
      (`ActorComponent.K2_DestroyComponent` (`self.Train`))
      (set `self.TrainDestroyed` true)
      (else
        (`/Engine/EditorBlueprintResources/StandardMacros.IsValid` (`self.RailroadRef`)
          (:`Is Valid`
            (if (not (`self.TrainDestroyed`))
              (`SceneComponent.K2_AddLocalOffset` (`self.Train`) (0.0 0.0 50.0) false false)
              (if (>= _returnvalue_y 5040.0)
                (`ActorComponent.K2_DestroyComponent` (`self.Train`))
                (set `self.TrainDestroyed` true)))))))))

(event `self.CollisionBox.OnComponentBeginOverlap`
  (params (OverlappedComponent :type "PrimitiveComponent Object Reference") (OtherActor :type "Actor Object Reference") (OtherComp :type "PrimitiveComponent Object Reference") (OtherBodyIndex :type Integer) (bFromSweep :type Boolean) (SweepResult :type "HitResult Structure (by ref)"))
  (bind _asbp_player (cast `/Game/Blueprints/BP_Player` OtherActor))
  (if (not (`/Game/Blueprints/BP_Player.ChickenDead` _asbp_player))
    (set `/Game/Blueprints/BP_Player.CannotMove` true _asbp_player)
    (`/Game/Blueprints/BP_Player.GameEnded` _asbp_player)))

(fn `UserConstructionScript`)