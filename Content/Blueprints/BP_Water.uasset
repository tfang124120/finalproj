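; BP_Water is a water lane for a chicken-crossing game that flags the player as on water and triggers its WaterSpawner to spawn land.
; BeginPlay randomly makes it either a lily-pad lane, filling unused spawn points, or a log lane with random side and speed.
; Delay-throttled Tick randomly spawns logs linked back to the lane, avoiding consecutive long ones.
; Wall overlaps make Tick push the chicken along negative X.
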(event `self.ReceiveBeginPlay`
  (`|MultiGate` true
    (:`Out 0`
      (`|MultiGate` true :!label _label
        (:`Out 0`
          (set `self.Spawn1` true))
        (:`Out 1`
          (set `self.Spawn2` true)))
      (`|MultiGate` true
        (:`Out 0`
          (set `self.Speed` (2.0 0.0 0.0)))
        (:`Out 1`
          (set `self.Speed` (4.0 0.0 0.0)))
        (:`Out 2`
          (set `self.Speed` (5.0 0.0 0.0)))))
    (:`Out 1`
      (goto _label))
    (:`Out 2`
      (goto _label))
    (:`Out 3`
      (`self.SpawnLilyPads`)
      (set `self.LilyPadsOnly` true))))

(event `self.ReceiveTick`
  (params (DeltaSeconds :type "Float (single-precision)"))
  (bind _returnvalue (`KismetMathLibrary.RandomInteger` 4))
  (`|ExecutionSequence`
    (:`then_0`
      (if (`self.Overlapped`)
        (bind _asbp_player (cast `/Game/Blueprints/BP_Player` (`GameplayStatics.GetPlayerCharacter` 0)))
        (`SceneComponent.K2_AddLocalOffset` (`/Game/Blueprints/BP_Player.RotateChicken` _asbp_player) (-15.0 0.0 0.0) false false)))
    (:`then_1`
      (if (not (`self.LilyPadsOnly`))
        (`KismetSystemLibrary.Delay` 1.5)
        (if (== _returnvalue 0)
          (if (`self.LongLogSpawned`)
            (`self.SpawnMediumLog` :!label _label_2)
            (set `self.LongLogSpawned` false)
            (else
              (`self.SpawnLongLog`)
              (set `self.LongLogSpawned` true)))
          (elif (== _returnvalue 1)
            (goto _label_2)
            (elif (== _returnvalue 2)
              (`self.SpawnSmallLog`)
              (set `self.LongLogSpawned` false))))))))

(event `self.TriggerZone.OnComponentBeginOverlap`
  (params (OverlappedComponent :type "PrimitiveComponent Object Reference") (OtherActor :type "Actor Object Reference") (OtherComp :type "PrimitiveComponent Object Reference") (OtherBodyIndex :type Integer) (bFromSweep :type Boolean) (SweepResult :type "HitResult Structure (by ref)"))
  (if (not (`self.Water Spawned`))
    (cast `/Game/Blueprints/BP_Player` OtherActor)
    (`/Engine/EditorBlueprintResources/StandardMacros.IsValid` (`self.Water Spawner`)
      (:`Is Valid`
        (`/Game/Blueprints/BP_SpawnLand.Spawn_Land at Spawn Point` (`self.Water Spawner`))
        (set `self.Water Spawned` true)))))

(event `self.DetectChicken.OnComponentBeginOverlap`
  (params (OverlappedComponent :type "PrimitiveComponent Object Reference") (OtherActor :type "Actor Object Reference") (OtherComp :type "PrimitiveComponent Object Reference") (OtherBodyIndex :type Integer) (bFromSweep :type Boolean) (SweepResult :type "HitResult Structure (by ref)"))
  (bind _asbp_player (cast `/Game/Blueprints/BP_Player` OtherActor))
  (set `/Game/Blueprints/BP_Player.IsOnWater` true _asbp_player))

(event `self.Wall1.OnComponentBeginOverlap`
  (params (OverlappedComponent :type "PrimitiveComponent Object Reference") (OtherActor :type "Actor Object Reference") (OtherComp :type "PrimitiveComponent Object Reference") (OtherBodyIndex :type Integer) (bFromSweep :type Boolean) (SweepResult :type "HitResult Structure (by ref)"))
  (cast `/Game/Blueprints/BP_Player` OtherActor)
  (set `self.Overlapped` true))

(event `self.Wall1.OnComponentEndOverlap`
  (params (OverlappedComponent :type "PrimitiveComponent Object Reference") (OtherActor :type "Actor Object Reference") (OtherComp :type "PrimitiveComponent Object Reference") (OtherBodyIndex :type Integer))
  (cast `/Game/Blueprints/BP_Player` OtherActor)
  (set `self.Overlapped` false))

(event `self.Wall2.OnComponentBeginOverlap`
  (params (OverlappedComponent :type "PrimitiveComponent Object Reference") (OtherActor :type "Actor Object Reference") (OtherComp :type "PrimitiveComponent Object Reference") (OtherBodyIndex :type Integer) (bFromSweep :type Boolean) (SweepResult :type "HitResult Structure (by ref)"))
  (cast `/Game/Blueprints/BP_Player` OtherActor)
  (set `self.Overlapped` true))

(event `self.Wall2.OnComponentEndOverlap`
  (params (OverlappedComponent :type "PrimitiveComponent Object Reference") (OtherActor :type "Actor Object Reference") (OtherComp :type "PrimitiveComponent Object Reference") (OtherBodyIndex :type Integer))
  (cast `/Game/Blueprints/BP_Player` OtherActor)
  (set `self.Overlapped` false))

(fn `SpawnLilyPads`
  (for _ (range 5)
    (`|MultiGate` true
      (:`Out 0`
        (if (`self.LilyPad1Spawned`) :!label _label
          (if (`self.LilyPad2Spawned`) :!label _label_2
            (if (`self.LilyPad3Spawned`) :!label _label_3
              (if (`self.LilyPad4Spawned`) :!label _label_4
                (if (`self.LilyPad5Spawned`) :!label _label_5
                  (if (`self.LilyPad6Spawned`) :!label _label_6
                    (if (`self.LilyPad7Spawned`) :!label _label_7
                      (if (`self.LilyPad8Spawned`) :!label _label_8
                        (if (`self.LilyPad9Spawned`) :!label _label_9
                          (if (`self.LilyPad10Spawned`) :!label _label_10
                            (if (`self.LilyPad11Spawned`) :!label _label_11
                              (if (`self.LilyPad12Spawned`) :!label _label_12
                                (if (`self.LilyPad13Spawned`) :!label _label_13
                                  (if (`self.LilyPad14Spawned`) :!label _label_14
                                    (if (`self.LilyPad15Spawned`) :!label _label_15
                                      (if (`self.LilyPad16Spawned`) :!label _label_16
                                        (goto _label)
                                        (else
                                          (set `self.LilyPadLocation` (`SceneComponent.K2_GetComponentLocation` (`self.LilyPadSpawn16`)))
                                          (set `self.LilyPad16Spawned` true)))
                                      (else
                                        (set `self.LilyPadLocation` (`SceneComponent.K2_GetComponentLocation` (`self.LilyPadSpawn15`)))
                                        (set `self.LilyPad15Spawned` true)))
                                    (else
                                      (set `self.LilyPadLocation` (`SceneComponent.K2_GetComponentLocation` (`self.LilyPadSpawn14`)))
                                      (set `self.LilyPad14Spawned` true)))
                                  (else
                                    (set `self.LilyPadLocation` (`SceneComponent.K2_GetComponentLocation` (`self.LilyPadSpawn13`)))
                                    (set `self.LilyPad13Spawned` true)))
                                (else
                                  (set `self.LilyPadLocation` (`SceneComponent.K2_GetComponentLocation` (`self.LilyPadSpawn12`)))
                                  (set `self.LilyPad12Spawned` true)))
                              (else
                                (set `self.LilyPadLocation` (`SceneComponent.K2_GetComponentLocation` (`self.LilyPadSpawn11`)))
                                (set `self.LilyPad11Spawned` true)))
                            (else
                              (set `self.LilyPadLocation` (`SceneComponent.K2_GetComponentLocation` (`self.LilyPadSpawn10`)))
                              (set `self.LilyPad10Spawned` true)))
                          (else
                            (set `self.LilyPadLocation` (`SceneComponent.K2_GetComponentLocation` (`self.LilyPadSpawn9`)))
                            (set `self.LilyPad9Spawned` true)))
                        (else
                          (set `self.LilyPadLocation` (`SceneComponent.K2_GetComponentLocation` (`self.LilyPadSpawn8`)))
                          (set `self.LilyPad8Spawned` true)))
                      (else
                        (set `self.LilyPadLocation` (`SceneComponent.K2_GetComponentLocation` (`self.LilyPadSpawn7`)))
                        (set `self.LilyPad7Spawned` true)))
                    (else
                      (set `self.LilyPadLocation` (`SceneComponent.K2_GetComponentLocation` (`self.LilyPadSpawn6`)))
                      (set `self.LilyPad6Spawned` true)))
                  (else
                    (set `self.LilyPadLocation` (`SceneComponent.K2_GetComponentLocation` (`self.LilyPadSpawn5`)))
                    (set `self.LilyPad5Spawned` true)))
                (else
                  (set `self.LilyPadLocation` (`SceneComponent.K2_GetComponentLocation` (`self.LilyPadSpawn4`)))
                  (set `self.LilyPad4Spawned` true)))
              (else
                (set `self.LilyPadLocation` (`SceneComponent.K2_GetComponentLocation` (`self.LilyPadSpawn3`)))
                (set `self.LilyPad3Spawned` true)))
            (else
              (set `self.LilyPadLocation` (`SceneComponent.K2_GetComponentLocation` (`self.LilyPadSpawn2`)))
              (set `self.LilyPad2Spawned` true)))
          (else
            (set `self.LilyPadLocation` (`SceneComponent.K2_GetComponentLocation` (`self.LilyPadSpawn1`)))
            (set `self.LilyPad1Spawned` true))))
      (:`Out 1`
        (goto _label_2))
      (:`Out 2`
        (goto _label_3))
      (:`Out 3`
        (goto _label_4))
      (:`Out 4`
        (goto _label_5))
      (:`Out 5`
        (goto _label_6))
      (:`Out 6`
        (goto _label_7))
      (:`Out 7`
        (goto _label_8))
      (:`Out 8`
        (goto _label_9))
      (:`Out 9`
        (goto _label_10))
      (:`Out 10`
        (goto _label_11))
      (:`Out 11`
        (goto _label_12))
      (:`Out 12`
        (goto _label_13))
      (:`Out 13`
        (goto _label_14))
      (:`Out 14`
        (goto _label_15))
      (:`Out 15`
        (goto _label_16)))
    (`|SpawnActorFromClass` "/Game/Blueprints/LilyPad.LilyPad_C" (`KismetMathLibrary.MakeTransform` (`self.LilyPadLocation`)) "Undefined" "OverrideRootScale" null null)))

(fn `SpawnLongLog`
  (if (`self.Spawn1`)
    (bind _returnvalue (`|SpawnActorFromClass` "/Game/Blueprints/BP_Longlog.BP_Longlog_C" (`KismetMathLibrary.MakeTransform` (`SceneComponent.K2_GetComponentLocation` (`self.LogSpawn1`))) "Undefined" "OverrideRootScale" null null))
    (set `/Game/Blueprints/BP_Longlog.WaterRef` self _returnvalue)
    (elif (`self.Spawn2`)
      (bind _returnvalue_2 (`|SpawnActorFromClass` "/Game/Blueprints/BP_Longlog.BP_Longlog_C" (`KismetMathLibrary.MakeTransform` (`SceneComponent.K2_GetComponentLocation` (`self.LogSpawn2`))) "Undefined" "OverrideRootScale" null null))
      (set `/Game/Blueprints/BP_Longlog.WaterRef` self _returnvalue_2))))

(fn `SpawnMediumLog`
  (if (`self.Spawn1`)
    (bind _returnvalue (`|SpawnActorFromClass` "/Game/Blueprints/BP_Mediumlog.BP_Mediumlog_C" (`KismetMathLibrary.MakeTransform` (`SceneComponent.K2_GetComponentLocation` (`self.LogSpawn1`))) "Undefined" "OverrideRootScale" null null))
    (set `/Game/Blueprints/BP_Mediumlog.WaterRef` self _returnvalue)
    (elif (`self.Spawn2`)
      (bind _returnvalue_2 (`|SpawnActorFromClass` "/Game/Blueprints/BP_Mediumlog.BP_Mediumlog_C" (`KismetMathLibrary.MakeTransform` (`SceneComponent.K2_GetComponentLocation` (`self.LogSpawn2`))) "Undefined" "OverrideRootScale" null null))
      (set `/Game/Blueprints/BP_Mediumlog.WaterRef` self _returnvalue_2))))

(fn `SpawnSmallLog`
  (if (`self.Spawn1`)
    (bind _returnvalue (`|SpawnActorFromClass` "/Game/Blueprints/BP_Smalllog.BP_Smalllog_C" (`KismetMathLibrary.MakeTransform` (`SceneComponent.K2_GetComponentLocation` (`self.LogSpawn1`))) "Undefined" "OverrideRootScale" null null))
    (set `/Game/Blueprints/BP_Smalllog.WaterRef` self _returnvalue)
    (elif (`self.Spawn2`)
      (bind _returnvalue_2 (`|SpawnActorFromClass` "/Game/Blueprints/BP_Smalllog.BP_Smalllog_C" (`KismetMathLibrary.MakeTransform` (`SceneComponent.K2_GetComponentLocation` (`self.LogSpawn2`))) "Undefined" "OverrideRootScale" null null))
      (set `/Game/Blueprints/BP_Smalllog.WaterRef` self _returnvalue_2))))

(fn `UserConstructionScript`)