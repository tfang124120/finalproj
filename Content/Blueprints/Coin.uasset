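; Coin is a pickup actor that adds one to the BP_Player's coin count when the player overlaps its Box.
; On pickup it destroys the Coin and Box components and sets CoinDestroyed, leaving the actor itself in place.
; Until then, Tick polls the player character's Restarting flag and removes both components the same way, without awarding a coin, when a restart is underway.
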(event `self.ReceiveTick`
  (params (DeltaSeconds :type "Float (single-precision)"))
  (if (not (`self.CoinDestroyed`))
    (bind _asbp_player (cast `/Game/Blueprints/BP_Player` (`GameplayStatics.GetPlayerCharacter` 0)))
    (if (`/Game/Blueprints/BP_Player.Restarting` _asbp_player)
      (`ActorComponent.K2_DestroyComponent` (`self.Coin`))
      (`ActorComponent.K2_DestroyComponent` (`self.Box`))
      (set `self.CoinDestroyed` true))))

(event `self.Box.OnComponentBeginOverlap`
  (params (OverlappedComponent :type "PrimitiveComponent Object Reference") (OtherActor :type "Actor Object Reference") (OtherComp :type "PrimitiveComponent Object Reference") (OtherBodyIndex :type Integer) (bFromSweep :type Boolean) (SweepResult :type "HitResult Structure (by ref)"))
  (`/Engine/EditorBlueprintResources/StandardMacros.IsValid` (`self.Coin`)
    (:`Is Valid`
      (bind _asbp_player (cast `/Game/Blueprints/BP_Player` OtherActor))
      (set `/Game/Blueprints/BP_Player.Coins` (+ (`/Game/Blueprints/BP_Player.Coins` _asbp_player) 1) _asbp_player)
      (`ActorComponent.K2_DestroyComponent` (`self.Coin`))
      (`ActorComponent.K2_DestroyComponent` (`self.Box`))
      (set `self.CoinDestroyed` true))))

(fn `UserConstructionScript`)