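; BP_LargeCar is a large road vehicle that kills the player's chicken on contact in a road-crossing game.
; Each Tick it moves at its RoadRef's Speed, turning 180 degrees once for Spawn2 roads.
; It destroys its mesh and transform components, not the actor, past the road's Y limit or on player restart.
; On overlap it squashes the chicken along an axis chosen by X offset, locks movement and calls GameEnded.
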(event `self.ReceiveBeginPlay`)

(event `self.ReceiveTick`
  (params (DeltaSeconds :type "Float (single-precision)"))
  (bind (_returnvalue_x _returnvalue_y) (`KismetMathLibrary.BreakVector` (`SceneComponent.K2_GetComponentLocation` (`self.TransformLargeCar`))))
  (bind (_returnvalue_x_2 _returnvalue_y_2) (`KismetMathLibrary.BreakVector` (`SceneComponent.K2_GetComponentLocation` (`self.TransformLargeCar`))))
  (if (not (`self.LargeCarDestroyed`))
    (bind _asbp_player (cast `/Game/Blueprints/BP_Player` (`GameplayStatics.GetPlayerCharacter` 0)))
    (if (`/Game/Blueprints/BP_Player.Restarting` _asbp_player)
      (`ActorComponent.K2_DestroyComponent` (`self.LargeCar`))
      (`ActorComponent.K2_DestroyComponent` (`self.TransformLargeCar`))
      (set `self.LargeCarDestroyed` true)
      (else
        (`/Engine/EditorBlueprintResources/StandardMacros.IsValid` (`self.RoadRef`)
          (:`Is Valid`
            (if (`/Game/Blueprints/BP_SingleRoad.Spawn1` (`self.RoadRef`))
              (`SceneComponent.K2_AddLocalOffset` (`self.TransformLargeCar`) (`/Game/Blueprints/BP_SingleRoad.Speed` (`self.RoadRef`)) false false)
              (if (>= _returnvalue_y_2 5040.0)
                (`ActorComponent.K2_DestroyComponent` (`self.TransformLargeCar`))
                (`ActorComponent.K2_DestroyComponent` (`self.LargeCar`))
                (set `self.LargeCarDestroyed` true))
              (elif (`/Game/Blueprints/BP_SingleRoad.Spawn2` (`self.RoadRef`))
                (if (`self.HasRotated`)
                  (`SceneComponent.K2_AddLocalOffset` (`self.TransformLargeCar`) (`/Game/Blueprints/BP_SingleRoad.Speed` (`self.RoadRef`)) false false)
                  (if (<= _returnvalue_y 0.0)
                    (`ActorComponent.K2_DestroyComponent` (`self.TransformLargeCar`))
                    (`ActorComponent.K2_DestroyComponent` (`self.LargeCar`))
                    (set `self.LargeCarDestroyed` true))
                  (else
                    (`SceneComponent.K2_AddLocalRotation` (`self.TransformLargeCar`) (struct :`Yaw` -180.0) false false)
                    (`SceneComponent.K2_AddLocalOffset` (`self.TransformLargeCar`) (`/Game/Blueprints/BP_SingleRoad.Speed` (`self.RoadRef`)) false false)
                    (set `self.HasRotated` true)))))))))))

(event `self.CollisionBox.OnComponentBeginOverlap`
  (params (OverlappedComponent :type "PrimitiveComponent Object Reference") (OtherActor :type "Actor Object Reference") (OtherComp :type "PrimitiveComponent Object Reference") (OtherBodyIndex :type Integer) (bFromSweep :type Boolean) (SweepResult :type "HitResult Structure (by ref)"))
  (bind _carhitlocation_x (`KismetMathLibrary.BreakVector` (`self.CarHitLocation`)))
  (bind _chickenhitlocation_x (`KismetMathLibrary.BreakVector` (`self.ChickenHitLocation`)))
  (bind _asbp_player (cast `/Game/Blueprints/BP_Player` OtherActor))
  (if (not (`/Game/Blueprints/BP_Player.ChickenDead` _asbp_player))
    (`/Engine/EditorBlueprintResources/StandardMacros.IsValid` (`self.TransformLargeCar`)
      (:`Is Valid`
        (set `self.CarHitLocation` (`SceneComponent.K2_GetComponentLocation` (`self.TransformLargeCar`)))
        (set `self.ChickenHitLocation` (`SceneComponent.K2_GetComponentLocation` (`/Game/Blueprints/BP_Player.RotateChicken` _asbp_player)))
        (if (>= (- _carhitlocation_x _chickenhitlocation_x) 10.0)
          (set `/Game/Blueprints/BP_Player.CannotMove` true _asbp_player)
          (bind _rotatechicken (`/Game/Blueprints/BP_Player.RotateChicken` _asbp_player))
          (`SceneComponent.K2_AddLocalTransform` _rotatechicken (`KismetMathLibrary.MakeTransform` (0.0 0.0 0.0) (struct) (0.5 2.25 2.25)) false false)
          (else
            (set `/Game/Blueprints/BP_Player.CannotMove` true _asbp_player)
            (`SceneComponent.K2_AddLocalTransform` _rotatechicken (`KismetMathLibrary.MakeTransform` (0.0 0.0 0.0) (struct) (2.25 2.25 0.5)) false false)))
        (`/Game/Blueprints/BP_Player.GameEnded` _asbp_player)))))

(fn `UserConstructionScript`)