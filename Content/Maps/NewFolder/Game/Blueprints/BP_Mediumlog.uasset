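; BP_Mediumlog is a medium floating log that carries the player's chicken across water.
; Each tick it moves by the referenced water's speed, in a direction set by Spawn1, and destroys its mesh component at either X limit or when the player restarts.
; Its trigger sets the player's on-log flag and log speed, clearing the flag on exit.
; A non-looping random MultiGate plays each landing sound at most once.
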(event `self.ReceiveBeginPlay`)

(event `self.ReceiveTick`
  (params (DeltaSeconds :type "Float (single-precision)"))
  (bind _returnvalue_x (`KismetMathLibrary.BreakVector` (`SceneComponent.K2_GetComponentLocation` (`self.Mediumlog`))))
  (bind _returnvalue_x_2 (`KismetMathLibrary.BreakVector` (`SceneComponent.K2_GetComponentLocation` (`self.Mediumlog`))))
  (if (not (`self.MediumLogDestroyed`))
    (bind _asbp_player (cast `/Game/Blueprints/BP_Player` (`GameplayStatics.GetPlayerCharacter` 0)))
    (if (`/Game/Blueprints/BP_Player.Restarting` _asbp_player)
      (`ActorComponent.K2_DestroyComponent` (`self.Mediumlog`))
      (set `self.MediumLogDestroyed` true)
      (elif (not (`self.MediumLogDestroyed`))
        (`/Engine/EditorBlueprintResources/StandardMacros.IsValid` (`self.WaterRef`)
          (:`Is Valid`
            (if (`/Game/Blueprints/BP_Water.Spawn1` (`self.WaterRef`))
              (bind _output_get (set `self.Speed` (`/Game/Blueprints/BP_Water.Speed` (`self.WaterRef`))))
              (`SceneComponent.K2_AddLocalOffset` (`self.Mediumlog`) _output_get false false)
              (if (>= _returnvalue_x 5040.0)
                (`ActorComponent.K2_DestroyComponent` (`self.Mediumlog`))
                (set `self.MediumLogDestroyed` true))
              (else
                (bind _output_get_2 (set `self.Speed` (`KismetMathLibrary.NegateVector` (`/Game/Blueprints/BP_Water.Speed` (`self.WaterRef`)))))
                (`SceneComponent.K2_AddLocalOffset` (`self.Mediumlog`) _output_get_2 false false)
                (if (<= _returnvalue_x_2 0.0)
                  (`ActorComponent.K2_DestroyComponent` (`self.Mediumlog`))
                  (set `self.MediumLogDestroyed` true))))))))))

(event `self.TriggerZone.OnComponentBeginOverlap`
  (params (OverlappedComponent :type "PrimitiveComponent Object Reference") (OtherActor :type "Actor Object Reference") (OtherComp :type "PrimitiveComponent Object Reference") (OtherBodyIndex :type Integer) (bFromSweep :type Boolean) (SweepResult :type "HitResult Structure (by ref)"))
  (bind _speed_x (`KismetMathLibrary.BreakVector` (`self.Speed`)))
  (bind _asbp_player (cast `/Game/Blueprints/BP_Player` OtherActor))
  (`|MultiGate` true
    (:`Out 0`
      (bind _returnvalue (`SceneComponent.K2_GetComponentLocation` (`/Game/Blueprints/BP_Player.RotateChicken` _asbp_player)))
      (`GameplayStatics.PlaySoundAtLocation` "/Game/Sounds/logjump3_Cue.logjump3_Cue" _returnvalue (struct) 1.0 1.0 0.0 null null null))
    (:`Out 1`
      (`GameplayStatics.PlaySoundAtLocation` "/Game/Sounds/logjump4_Cue.logjump4_Cue" _returnvalue (struct) 1.0 1.0 0.0 null null null)))
  (set `/Game/Blueprints/BP_Player.ChickenOnLog` true _asbp_player)
  (set `/Game/Blueprints/BP_Player.LogSpeed` (`KismetMathLibrary.MakeVector` 0.0 _speed_x) _asbp_player))

(event `self.TriggerZone.OnComponentEndOverlap`
  (params (OverlappedComponent :type "PrimitiveComponent Object Reference") (OtherActor :type "Actor Object Reference") (OtherComp :type "PrimitiveComponent Object Reference") (OtherBodyIndex :type Integer))
  (bind _asbp_player (cast `/Game/Blueprints/BP_Player` OtherActor))
  (set `/Game/Blueprints/BP_Player.ChickenOnLog` false _asbp_player))

(fn `UserConstructionScript`)