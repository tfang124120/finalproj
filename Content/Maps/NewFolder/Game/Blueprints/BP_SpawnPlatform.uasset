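; BP_SpawnPlatform is a platform actor that triggers land spawning and drifts the player's RotateChicken component.
; Entering TriggerZone calls SpawnLandAtSpawnPoint on a valid RoadSpawner, with RoadSpawned limiting it to one spawn.
; While the player overlaps the actor, Tick shifts RotateChicken along negative local X by a fixed per-frame step, not scaled by delta time.
; Being inside TriggerZone sets Override, which suspends that drift until exit.
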(event `self.ReceiveTick`
  (params (DeltaSeconds :type "Float (single-precision)"))
  (if (`self.Override`)
    _
    (elif (`self.Overlapped`)
      (bind _asbp_player (cast `/Game/Blueprints/BP_Player` (`GameplayStatics.GetPlayerCharacter` 0)))
      (`SceneComponent.K2_AddLocalOffset` (`/Game/Blueprints/BP_Player.RotateChicken` _asbp_player) (-15.0 0.0 0.0) false false))))

(event `self.TriggerZone.OnComponentBeginOverlap`
  (params (OverlappedComponent :type "PrimitiveComponent Object Reference") (OtherActor :type "Actor Object Reference") (OtherComp :type "PrimitiveComponent Object Reference") (OtherBodyIndex :type Integer) (bFromSweep :type Boolean) (SweepResult :type "HitResult Structure (by ref)"))
  (cast `/Game/Blueprints/BP_Player` OtherActor)
  (set `self.Override` true)
  (if (not (`self.RoadSpawned`))
    (`/Engine/EditorBlueprintResources/StandardMacros.IsValid` (`self.RoadSpawner`)
      (:`Is Valid`
        (`/Game/Blueprints/BP_SpawnLand.Spawn_Land at Spawn Point` (`self.RoadSpawner`))
        (set `self.RoadSpawned` true)))))

(event `self.TriggerZone.OnComponentEndOverlap`
  (params (OverlappedComponent :type "PrimitiveComponent Object Reference") (OtherActor :type "Actor Object Reference") (OtherComp :type "PrimitiveComponent Object Reference") (OtherBodyIndex :type Integer))
  (cast `/Game/Blueprints/BP_Player` OtherActor)
  (set `self.Override` false))

(event `self.ReceiveActorBeginOverlap`
  (params (OtherActor :type "Actor Object Reference"))
  (cast `/Game/Blueprints/BP_Player` OtherActor)
  (set `self.Overlapped` true))

(event `self.ReceiveActorEndOverlap`
  (params (OtherActor :type "Actor Object Reference"))
  (cast `/Game/Blueprints/BP_Player` OtherActor)
  (set `self.Overlapped` false))

(fn `UserConstructionScript`)