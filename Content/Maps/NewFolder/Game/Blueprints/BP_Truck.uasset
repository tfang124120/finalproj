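; Truck obstacle that drives along a road and kills the player's chicken on contact.
; Each Tick it moves by its road's Speed, turning 180 degrees once for the second spawn side.
; It destroys its components, not the actor, past the road's Y limit or when the player restarts.
; On overlap with a living chicken, it blocks movement, distorts the chicken's scale based on relative X position and calls GameEnded.
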(event `self.ReceiveTick`
  (params (DeltaSeconds :type "Float (single-precision)"))
  (bind (_returnvalue_x _returnvalue_y) (`KismetMathLibrary.BreakVector` (`SceneComponent.K2_GetComponentLocation` (`self.TransformTruck`))))
  (bind (_returnvalue_x_2 _returnvalue_y_2) (`KismetMathLibrary.BreakVector` (`SceneComponent.K2_GetComponentLocation` (`self.TransformTruck`))))
  (if (not (`self.TruckDestroyed`))
    (bind _asbp_player (cast `/Game/Blueprints/BP_Player` (`GameplayStatics.GetPlayerCharacter` 0)))
    (if (`/Game/Blueprints/BP_Player.Restarting` _asbp_player)
      (`ActorComponent.K2_DestroyComponent` (`self.TransformTruck`))
      (`ActorComponent.K2_DestroyComponent` (`self.Truck`))
      (set `self.TruckDestroyed` true)
      (else
        (`/Engine/EditorBlueprintResources/StandardMacros.IsValid` (`self.RoadRef`)
          (:`Is Valid`
            (if (`self.TruckDestroyed`)
              _
              (elif (`/Game/Blueprints/BP_SingleRoad.Spawn1` (`self.RoadRef`))
                (`SceneComponent.K2_AddLocalTransform` (`self.TransformTruck`) (`KismetMathLibrary.MakeTransform` (`/Game/Blueprints/BP_SingleRoad.Speed` (`self.RoadRef`))) false false)
                (if (>= _returnvalue_y 5040.0)
                  (`ActorComponent.K2_DestroyComponent` (`self.TransformTruck`))
                  (`ActorComponent.K2_DestroyComponent` (`self.Truck`))
                  (set `self.TruckDestroyed` true))
                (elif (`/Game/Blueprints/BP_SingleRoad.Spawn2` (`self.RoadRef`))
                  (if (`self.HasRotated`)
                    (`SceneComponent.K2_AddLocalOffset` (`self.TransformTruck`) (`/Game/Blueprints/BP_SingleRoad.Speed` (`self.RoadRef`)) false false)
                    (if (<= _returnvalue_y_2 0.0)
                      (`ActorComponent.K2_DestroyComponent` (`self.TransformTruck`))
                      (`ActorComponent.K2_DestroyComponent` (`self.Truck`))
                      (set `self.TruckDestroyed` true))
                    (else
                      (`SceneComponent.K2_AddLocalTransform` (`self.TransformTruck`) (`KismetMathLibrary.MakeTransform` (`/Game/Blueprints/BP_SingleRoad.Speed` (`self.RoadRef`)) (struct :`Yaw` -180.0)) false false)
                      (set `self.HasRotated` true))))))))))))

(event `self.CollisionBox.OnComponentBeginOverlap`
  (params (OverlappedComponent :type "PrimitiveComponent Object Reference") (OtherActor :type "Actor Object Reference") (OtherComp :type "PrimitiveComponent Object Reference") (OtherBodyIndex :type Integer) (bFromSweep :type Boolean) (SweepResult :type "HitResult Structure (by ref)"))
  (bind _truckhitlocation_x (`KismetMathLibrary.BreakVector` (`self.TruckHitLocation`)))
  (bind _chickenhitlocation_x (`KismetMathLibrary.BreakVector` (`self.ChickenHitLocation`)))
  (bind _asbp_player (cast `/Game/Blueprints/BP_Player` OtherActor))
  (if (not (`/Game/Blueprints/BP_Player.ChickenDead` _asbp_player))
    (`/Engine/EditorBlueprintResources/StandardMacros.IsValid` (`self.TransformTruck`)
      (:`Is Valid`
        (set `self.TruckHitLocation` (`SceneComponent.K2_GetComponentLocation` (`self.TransformTruck`)))
        (set `self.ChickenHitLocation` (`SceneComponent.K2_GetComponentLocation` (`/Game/Blueprints/BP_Player.RotateChicken` _asbp_player)))
        (if (>= (- _truckhitlocation_x _chickenhitlocation_x) 10.0)
          (set `/Game/Blueprints/BP_Player.CannotMove` true _asbp_player)
          (bind _rotatechicken (`/Game/Blueprints/BP_Player.RotateChicken` _asbp_player))
          (`SceneComponent.K2_AddLocalTransform` _rotatechicken (`KismetMathLibrary.MakeTransform` (0.0 0.0 0.0) (struct) (0.5 2.25 2.25)) false false)
          (else
            (set `/Game/Blueprints/BP_Player.CannotMove` true _asbp_player)
            (`SceneComponent.K2_AddLocalTransform` _rotatechicken (`KismetMathLibrary.MakeTransform` (0.0 0.0 0.0) (struct) (2.25 2.25 0.5)) false false)))
        (`/Game/Blueprints/BP_Player.GameEnded` _asbp_player)))))

(fn `UserConstructionScript`)